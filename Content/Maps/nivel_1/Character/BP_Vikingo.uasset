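; BP_Vikingo is the player Viking character, with Enhanced Input movement, look, jump and dash.
; It registers its mapping context on BeginPlay, then moves along world X, snapping control yaw to 0 or 180 by acceleration direction, as in a side-scroller.
; Jump also calls a montage; dash launches along forward X, gated by a DoOnce that resets after a short delay.
; Interact and hammer-throw inputs are empty stubs, and an upward launch is left disconnected.
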(event `self.ReceiveBeginPlay`
  (bind _asplayer_controller (cast `PlayerController` (`self.GetController`)))
  (`EnhancedInputSubsystemInterface.AddMappingContext` (pcsubsystem `EnhancedInputLocalPlayerSubsystem` _asplayer_controller) "/Game/Maps/nivel_1/Character/imputs/Mapping/IMC_Character.IMC_Character" 0 (struct)))

(event `EnhancedInput|/Game/Maps/nivel_1/Character/imputs/IA_Mirar`
  (params (ActionValue :type "Float (double-precision)") (ElapsedSeconds :type "Float (double-precision)") (TriggeredSeconds :type "Float (double-precision)") (InputAction :type "InputAction Object Reference" :default "/Game/Maps/nivel_1/Character/imputs/IA_Mirar.IA_Mirar"))
  (:`Triggered`
    (`self.AddControllerYawInput` ActionValue)))

(event `EnhancedInput|/Game/Maps/nivel_1/Character/imputs/IA_Movimiento`
  (params (ActionValue :type "Float (double-precision)") (ElapsedSeconds :type "Float (double-precision)") (TriggeredSeconds :type "Float (double-precision)") (InputAction :type "InputAction Object Reference" :default "/Game/Maps/nivel_1/Character/imputs/IA_Movimiento.IA_Movimiento"))
  (bind _returnvalue (`self.GetController`))
  (bind _returnvalue_x (`KismetMathLibrary.BreakVector` (`CharacterMovementComponent.GetCurrentAcceleration` (`self.CharacterMovement`))))
  (:`Triggered`
    (`self.AddMovementInput` (1.0 0.0 0.0) ActionValue)
    (`/Engine/EditorBlueprintResources/StandardMacros.CompareFloat` _returnvalue_x
      (:`>`
        (`Controller.SetControlRotation` _returnvalue (`KismetMathLibrary.MakeRotator` 0.0)))
      (:`<`
        (`Controller.SetControlRotation` _returnvalue (`KismetMathLibrary.MakeRotator` 0.0 0.0 180.0))))))

(event `EnhancedInput|/Game/Maps/nivel_1/Character/imputs/IA_saltar`
  (params (ActionValue :type "Float (double-precision)") (ElapsedSeconds :type "Float (double-precision)") (TriggeredSeconds :type "Float (double-precision)") (InputAction :type "InputAction Object Reference" :default "/Game/Maps/nivel_1/Character/imputs/IA_saltar.IA_saltar"))
  (:`Started`
    (`self.Jump`)
    (`self.PlayAnimMontage` null)))

(event `EnhancedInput|/Game/Maps/nivel_1/Character/imputs/IA_Dash`
  (params (ActionValue :type Boolean) (ElapsedSeconds :type "Float (double-precision)") (TriggeredSeconds :type "Float (double-precision)") (InputAction :type "InputAction Object Reference" :default "/Game/Maps/nivel_1/Character/imputs/IA_Dash.IA_Dash"))
  (:`Started`
    (`/Engine/EditorBlueprintResources/StandardMacros.DoOnce` false :!label _label
      (:`Completed`
        (`self.LaunchCharacter` (* (`self.GetActorForwardVector`) (1000.0 0.0 0.0)))
        (`KismetSystemLibrary.Delay` 0.1)
        (goto _label :!via `Reset`)))))

(event `EnhancedInput|/Game/Maps/nivel_1/Character/imputs/IA_interactuar`
  (params (ActionValue :type Boolean) (ElapsedSeconds :type "Float (double-precision)") (TriggeredSeconds :type "Float (double-precision)") (InputAction :type "InputAction Object Reference" :default "/Game/Maps/nivel_1/Character/imputs/IA_interactuar.IA_interactuar")))

(event `EnhancedInput|/Game/Maps/nivel_1/Character/imputs/IA_Lanzar_Martillo`
  (params (ActionValue :type "Float (double-precision)") (ElapsedSeconds :type "Float (double-precision)") (TriggeredSeconds :type "Float (double-precision)") (InputAction :type "InputAction Object Reference" :default "/Game/Maps/nivel_1/Character/imputs/IA_Lanzar_Martillo.IA_Lanzar_Martillo")))

(fn `UserConstructionScript`)