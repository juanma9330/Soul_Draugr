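; Player character with side-scroller style movement along world X, flipping control yaw to face the direction of travel.
; Enhanced Input drives looking, jump, run, crouch, potion healing, quitting, and launch-based dash and slide.
; Events handle key, coin and potion pickups plus area damage and healing, printing debug text.
; Tick calls Muerte and respawns the character when health runs out; hammer throw and interact inputs do nothing.
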(event `self.ReceiveBeginPlay`
  (bind _asplayer_controller (cast `PlayerController` (`self.GetController`)))
  (`EnhancedInputSubsystemInterface.AddMappingContext` (pcsubsystem `EnhancedInputLocalPlayerSubsystem` _asplayer_controller) "/Game/Maps/nivel_1/Character/imputs/Mapping/IMC_Character.IMC_Character" 0 (struct)))

(event `EnhancedInput|/Game/Maps/nivel_1/Character/imputs/IA_Mirar`
  (params (ActionValue :type "Float (double-precision)") (ElapsedSeconds :type "Float (double-precision)") (TriggeredSeconds :type "Float (double-precision)") (InputAction :type "InputAction Object Reference" :default "/Game/Maps/nivel_1/Character/imputs/IA_Mirar.IA_Mirar"))
  ;[1 1 1] Mirar
  (:`Triggered`
    (`self.AddControllerYawInput` ActionValue)))

(event `EnhancedInput|/Game/Maps/nivel_1/Character/imputs/IA_Movimiento`
  (params (ActionValue :type "Float (double-precision)") (ElapsedSeconds :type "Float (double-precision)") (TriggeredSeconds :type "Float (double-precision)") (InputAction :type "InputAction Object Reference" :default "/Game/Maps/nivel_1/Character/imputs/IA_Movimiento.IA_Movimiento"))
  (bind _returnvalue (`self.GetController`))
  (bind _returnvalue_x (`KismetMathLibrary.BreakVector` (`CharacterMovementComponent.GetCurrentAcceleration` (`self.CharacterMovement`))))
  ;[1 1 1] Movimiento
  (:`Triggered`
    (`self.AddMovementInput` (1.0 0.0 0.0) ActionValue)
    (`/Engine/EditorBlueprintResources/StandardMacros.CompareFloat` _returnvalue_x
      (:`>`
        (`Controller.SetControlRotation` _returnvalue (`KismetMathLibrary.MakeRotator` 0.0)))
      (:`<`
        (`Controller.SetControlRotation` _returnvalue (`KismetMathLibrary.MakeRotator` 0.0 0.0 180.0))))))

(event `EnhancedInput|/Game/Maps/nivel_1/Character/imputs/IA_saltar`
  (params (ActionValue :type Boolean) (ElapsedSeconds :type "Float (double-precision)") (TriggeredSeconds :type "Float (double-precision)") (InputAction :type "InputAction Object Reference" :default "/Game/Maps/nivel_1/Character/imputs/IA_saltar.IA_saltar"))
  ;[1 1 1] Salto
  (:`Started`
    (`self.Jump`)
    (`KismetSystemLibrary.Delay` 0.7))
  (:`Completed`
    (`self.StopJumping`)))

(event `EnhancedInput|/Game/Maps/nivel_1/Character/imputs/IA_Dash`
  (params (ActionValue :type Boolean) (ElapsedSeconds :type "Float (double-precision)") (TriggeredSeconds :type "Float (double-precision)") (InputAction :type "InputAction Object Reference" :default "/Game/Maps/nivel_1/Character/imputs/IA_Dash.IA_Dash"))
  (bind _returnvalue_x (`KismetMathLibrary.BreakVector` (* (`self.GetVelocity`) (`self.Velocidad dash`))))
  ;[1 1 1] Dash
  (:`Started`
    (`self.LaunchCharacter` (`KismetMathLibrary.MakeVector` _returnvalue_x))
    (`KismetSystemLibrary.Delay` 0.7)))

(event `EnhancedInput|/Game/Maps/nivel_1/Character/imputs/IA_Correr`
  (params (ActionValue :type "Float (double-precision)") (ElapsedSeconds :type "Float (double-precision)") (TriggeredSeconds :type "Float (double-precision)") (InputAction :type "InputAction Object Reference" :default "/Game/Maps/nivel_1/Character/imputs/IA_Correr.IA_Correr"))
  (bind _charactermovement (`self.CharacterMovement`))
  ;[1 1 1] correr
  (:`Started`
    (set `CharacterMovementComponent.MaxWalkSpeed` (* (`CharacterMovementComponent.MaxWalkSpeed` _charactermovement) 3.0) _charactermovement))
  (:`Completed`
    (set `CharacterMovementComponent.MaxWalkSpeed` 600.0 (`self.CharacterMovement`))))

(event `EnhancedInput|/Game/Maps/nivel_1/Character/imputs/IA_Agacharse`
  (params (ActionValue :type Boolean) (ElapsedSeconds :type "Float (double-precision)") (TriggeredSeconds :type "Float (double-precision)") (InputAction :type "InputAction Object Reference" :default "/Game/Maps/nivel_1/Character/imputs/IA_Agacharse.IA_Agacharse"))
  ;[1 1 1] agacharse
  (:`Started`
    (`self.Crouch`))
  (:`Completed`
    (`self.UnCrouch`)))

(event `EnhancedInput|/Game/Maps/nivel_1/Character/imputs/IA_DeslizarsePorElSuelo`
  (params (ActionValue :type Boolean) (ElapsedSeconds :type "Float (double-precision)") (TriggeredSeconds :type "Float (double-precision)") (InputAction :type "InputAction Object Reference" :default "/Game/Maps/nivel_1/Character/imputs/IA_DeslizarsePorElSuelo.IA_DeslizarsePorElSuelo"))
  (bind _returnvalue_x (`KismetMathLibrary.BreakVector` (`self.GetVelocity`)))
  ;[1 1 1] deslizamiento por el suelo
  (:`Started`
    (if (not (`NavMovementComponent.IsFalling` (`self.CharacterMovement`)))
      (`self.Crouch`)
      (`self.LaunchCharacter` (`KismetMathLibrary.MakeVector` (* _returnvalue_x 15.0)))
      (`KismetSystemLibrary.Delay` 0.7)))
  (:`Completed`
    (`self.UnCrouch`)))

(event `EnhancedInput|/Game/Maps/nivel_1/Character/imputs/IA_Quit_Game`
  (params (ActionValue :type Boolean) (ElapsedSeconds :type "Float (double-precision)") (TriggeredSeconds :type "Float (double-precision)") (InputAction :type "InputAction Object Reference" :default "/Game/Maps/nivel_1/Character/imputs/IA_Quit_Game.IA_Quit_Game"))
  ;[1 1 1] Cerrar juego
  (:`Started`
    (`KismetSystemLibrary.QuitGame` null "Quit" true)))

(event `EnhancedInput|/Game/Maps/nivel_1/Character/imputs/IA_Curarse`
  (params (ActionValue :type Boolean) (ElapsedSeconds :type "Float (double-precision)") (TriggeredSeconds :type "Float (double-precision)") (InputAction :type "InputAction Object Reference" :default "/Game/Maps/nivel_1/Character/imputs/IA_Curarse.IA_Curarse"))
  ;[1 1 1] Curarse con poción
  (:`Started`
    (`self.TomarPoción` (`self.Curación de poción`))))

(event `EnhancedInput|/Game/Maps/nivel_1/Character/imputs/IA_Lanzar_Martillo`
  (params (ActionValue :type Boolean) (ElapsedSeconds :type "Float (double-precision)") (TriggeredSeconds :type "Float (double-precision)") (InputAction :type "InputAction Object Reference" :default "/Game/Maps/nivel_1/Character/imputs/IA_Lanzar_Martillo.IA_Lanzar_Martillo")))

(event `EnhancedInput|/Game/Maps/nivel_1/Character/imputs/IA_interactuar`
  (params (ActionValue :type Boolean) (ElapsedSeconds :type "Float (double-precision)") (TriggeredSeconds :type "Float (double-precision)") (InputAction :type "InputAction Object Reference" :default "/Game/Maps/nivel_1/Character/imputs/IA_interactuar.IA_interactuar")))

(event `/Game/Maps/Interfase/Bpi_ObtenerLlave.ObtenerLlave`
  (params (LLaves :type Integer))
  ;[1 1 1] Obtener Llave
  (bind _output_get (set `self.LLave` (+ LLaves (`self.LLave`))))
  (`KismetSystemLibrary.PrintString` (`KismetStringLibrary.Concat_StrStr` "Número de Llaves" (`KismetStringLibrary.Conv_IntToString` _output_get)) true true (struct :`R` 1.0 :`G` 0.465167 :`B` 0.052083 :`A` 1.0) 5.0))

(event `/Game/Maps/Interfase/Bpi_Recolectar.Obtener_Monedas`
  (params (Monedas :type Integer))
  ;[1 1 1] obtener monedas
  (bind _output_get (set `self.Monedas` (+ Monedas (`self.Monedas`))))
  (`KismetSystemLibrary.PrintString` (`KismetStringLibrary.Concat_StrStr` "Número de monedas totales: \n" (`KismetStringLibrary.Conv_IntToString` _output_get)) true true (struct :`R` 0.997933 :`G` 1.0 :`A` 1.0) 5.0))

(event `/Game/Maps/Interfase/Bpi_ObtenerPociónDeCuración.ObtenerPociónCuración`
  (params (Pociones :type Integer))
  ;[1 1 1] Obtener pociones
  (bind _output_get (set `self.Pociones` (+ Pociones (`self.Pociones`))))
  (`KismetSystemLibrary.PrintString` (`KismetStringLibrary.Concat_StrStr` "Número de pociones totales: \n" (`KismetStringLibrary.Conv_IntToString` _output_get)) true true (struct :`R` 0.997933 :`G` 1.0 :`A` 1.0) 5.0))

(event `/Game/Maps/Interfase/Bpi_DañoDeArea.DañoDeÁrea`
  (params (`DañoDeÁrea` :type "Float (double-precision)"))
  ;[1 1 1] zona de daño
  (bind _output_get (set `self.Vida` (- (`self.Vida`) `DañoDeÁrea`)))
  (`KismetSystemLibrary.PrintString` (`KismetStringLibrary.Concat_StrStr` "Vida \n" (`KismetStringLibrary.Conv_DoubleToString` _output_get)) true true (struct :`R` 0.549777 :`G` 0.114425 :`B` 0.864583 :`A` 1.0) 5.0 "Salud"))

(event `/Game/Maps/Interfase/Bpi_ZonaDeCuración.ZonaCuración`
  (params (`Curación` :type "Float (double-precision)"))
  ;[1 1 1] Zona de curación
  (bind _output_get (set `self.Vida` (+ `Curación` (`self.Vida`))))
  (if (> _output_get (`self.VidaMaxima`))
    (bind _output_get_2 (set `self.Vida` (`self.VidaMaxima`)))
    (`KismetSystemLibrary.PrintString` (`KismetStringLibrary.Concat_StrStr` "Vida \n" (`KismetStringLibrary.Conv_DoubleToString` _output_get_2)) true true (struct :`R` 0.549777 :`G` 0.114425 :`B` 0.864583 :`A` 1.0) 10.0 "Salud")))

(event `/Game/Maps/Interfase/Bpi_TomarPociónDeCuración.TomarPoción`
  (params (Curarse :type "Float (double-precision)"))
  (bind _vida (`self.Vida`))
  (bind _pociones (`self.Pociones`))
  ;[1 1 1] Curación con poción
  (if (and (>= _pociones 1) (< _vida (`self.VidaMaxima`)))
    (set `self.Vida` (+ Curarse (`self.Vida`)))
    (bind _output_get (set `self.Pociones` (- (`self.Pociones`) 1)))
    (if (> (`self.Vida`) (`self.VidaMaxima`))
      (bind _output_get_2 (set `self.Vida` (`self.VidaMaxima`)))
      (`KismetSystemLibrary.PrintString` (`KismetStringLibrary.Concat_StrStr` "Vida:    " (`KismetStringLibrary.Conv_DoubleToString` _output_get_2) " \nCantidad de pociones:   " (`KismetStringLibrary.Conv_IntToString` _output_get)) true true (struct :`R` 0.549777 :`G` 0.114425 :`B` 0.864583 :`A` 1.0) 50.0 "None"))
    (else
      (`KismetSystemLibrary.PrintString` (`KismetStringLibrary.Concat_StrStr` "Vida:    " (`KismetStringLibrary.Conv_DoubleToString` _vida) " \nCantidad de pociones:   " (`KismetStringLibrary.Conv_IntToString` _pociones))))))

(event `self.ReceiveTick`
  (params (DeltaSeconds :type "Float (single-precision)"))
  (if (<= (`self.Vida`) 0.0)
    (`self.Muerte`)
    (`self.K2_SetActorLocation` (`self.Posición de respawn`) false true)
    (set `self.Vida` (`self.Vida inicial`))))

(fn `UserConstructionScript`)